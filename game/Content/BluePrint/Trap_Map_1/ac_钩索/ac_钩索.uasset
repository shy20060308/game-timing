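; Grappling hook component for a player character that pulls it to the targeted anchor point.
; Anchors are added to or removed from an array; each Tick picks the one best aligned with the controller's forward vector, above a dot threshold, and toggles its target state.
; Pressing T turns the character, moves it above the anchor at distance-based timing, spawns a Niagara rope from the hand, then zeroes velocity on arrival.
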(event `self.ReceiveBeginPlay`
  (bind `_as角色` (cast `Character` (`self.GetOwner`)))
  (set `self.As角色` `_as角色`)
  (bind `_as玩家控制器` (cast `PlayerController` (`Pawn.GetController` `_as角色`)))
  (set `self.As玩家控制器` `_as玩家控制器`))

(event `self.ReceiveTick`
  (params (DeltaSeconds :type "Float (single-precision)"))
  (bind `_当前锚点` (`self.当前锚点`))
  (bind `_新锚点` (`self.锚点检测`))
  (if (not (== `_新锚点` (`self.当前锚点`)))
    (`/Engine/EditorBlueprintResources/StandardMacros.IsValid` `_当前锚点`
      (:`Is Valid`
        (`/Game/BluePrint/Trap_Map_1/ac_钩索/bp_钩索锚点.退出目标锚点` `_当前锚点`))
      (:`Is Not Valid`
        _))
    (bind _output_get (set `self.当前锚点` `_新锚点`))
    (`/Engine/EditorBlueprintResources/StandardMacros.IsValid` _output_get
      (:`Is Valid`
        (`/Game/BluePrint/Trap_Map_1/ac_钩索/bp_钩索锚点.设为目标锚点` _output_get)))))

(event `添加到组件`
  (params (NewItem :type "/Game/BluePrint/Trap_Map_1/ac_钩索/bp_钩索锚点 Object Reference (by ref)"))
  (`KismetArrayLibrary.Array_Add` (`self.钩索数组`) NewItem))

(event `从组件移除`
  (params (Item :type "/Game/BluePrint/Trap_Map_1/ac_钩索/bp_钩索锚点 Object Reference (by ref)"))
  (`KismetArrayLibrary.Array_RemoveItem` (`self.钩索数组`) Item))

(event `Key|T`
  (params (Key :type "Key Structure"))
  (:`Pressed`
    (`/Engine/EditorBlueprintResources/StandardMacros.IsValid` (`self.当前锚点`)
      (:`Is Valid`
        (`self.角色转向`)
        (`self.角色移动`)
        (bind _returnvalue (`NiagaraFunctionLibrary.SpawnSystemAttached` "/Game/BluePrint/Trap_Map_1/ac_钩索/vfx/NewNiagaraSystem.NewNiagaraSystem" (`Character.Mesh` (`self.As角色`)) "hand_r" (0.0 0.0 0.0) (struct) "KeepRelativeOffset"))
        (`NiagaraComponent.SetVariableVec3` _returnvalue "end" (`Actor.K2_GetActorLocation` (`self.当前锚点`)))
        (`NiagaraComponent.SetVariableFloat` _returnvalue "lifetime" (/ (`KismetMathLibrary.Vector_Distance` (`Actor.K2_GetActorLocation` (`self.As角色`)) (`Actor.K2_GetActorLocation` (`self.当前锚点`))) (`self.钩索移动速度`)))))))

(event `角色转向`
  (bind (_returnvalue_roll _returnvalue_pitch _returnvalue_yaw) (`KismetMathLibrary.BreakRotator` (`KismetMathLibrary.FindLookAtRotation` (`Actor.K2_GetActorLocation` (`self.As角色`)) (`Actor.K2_GetActorLocation` (`self.当前锚点`)))))
  (`Actor.K2_SetActorRotation` (`self.As角色`) (`KismetMathLibrary.MakeRotator` 0.0 0.0 _returnvalue_yaw) false))

(event `角色移动`
  (bind `_当前锚点` (`self.当前锚点`))
  (bind (_returnvalue_x _returnvalue_y _returnvalue_z) (`KismetMathLibrary.BreakVector` (`Actor.K2_GetActorLocation` `_当前锚点`)))
  (bind _returnvalue (/ (`KismetMathLibrary.Vector_Distance` (`Actor.K2_GetActorLocation` (`self.As角色`)) (`Actor.K2_GetActorLocation` `_当前锚点`)) (`self.钩索移动速度`)))
  (`|ExecutionSequence`
    (:`then_0`
      (`KismetSystemLibrary.MoveComponentTo` (`Actor.RootComponent` (`self.As角色`)) (`KismetMathLibrary.MakeVector` _returnvalue_x _returnvalue_y (+ _returnvalue_z 100.0)) (`Actor.K2_GetActorRotation` (`self.As角色`)) false false _returnvalue))
    (:`then_1`
      (`KismetSystemLibrary.Delay` _returnvalue)
      (set `MovementComponent.Velocity` (0.0 0.0 0.0) (`Character.CharacterMovement` (`self.As角色`))))))

(fn `角度判断`
  (params (`钩索actor` :type "/Game/BluePrint/Trap_Map_1/ac_钩索/bp_钩索锚点 Object Reference"))
  (returns (ReturnValue :type "Float (double-precision)"))
  (return (`KismetMathLibrary.Dot_VectorVector` (`Actor.GetActorForwardVector` (`self.As玩家控制器`)) (`KismetMathLibrary.GetDirectionUnitVector` (`Actor.K2_GetActorLocation` (`self.As角色`)) (`Actor.K2_GetActorLocation` `钩索actor`)))))

(fn `锚点检测`
  (returns (`新锚点` :type "/Game/BluePrint/Trap_Map_1/ac_钩索/bp_钩索锚点 Object Reference"))
  (locals (`和锚点夹角` :type "Float (double-precision)") (`目标锚点` :type "/Game/BluePrint/Trap_Map_1/ac_钩索/bp_钩索锚点 Object Reference"))
  (`/Engine/EditorBlueprintResources/StandardMacros.DoOnce` false :!label _label
    (:`Completed`
      (set `local.和锚点夹角` 0.3)
      (set `local.目标锚点` null)
      (for _array_element (`self.钩索数组`)
        (bind _returnvalue (`self.角度判断` _array_element))
        (if (> _returnvalue (`local.和锚点夹角`))
          (set `local.和锚点夹角` _returnvalue)
          (set `local.目标锚点` _array_element)))
      (`|ExecutionSequence`
        (:`then_0`
          (return (`local.目标锚点`)))
        (:`then_1`
          (goto _label :!via `Reset`))))))