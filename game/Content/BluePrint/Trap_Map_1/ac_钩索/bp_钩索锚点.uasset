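; Grappling hook anchor point (钩索锚点) that actors carrying the Ac_钩索 component can detect as a candidate target.
; Overlapping its Sphere1 registers the anchor with that actor's component, and leaving the sphere removes it.
; Two events, for becoming and ceasing to be the target anchor, swap the material on Sphere to show the targeted state.
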(event `self.Sphere1.OnComponentBeginOverlap`
  (params (OverlappedComponent :type "PrimitiveComponent Object Reference") (OtherActor :type "Actor Object Reference") (OtherComp :type "PrimitiveComponent Object Reference") (OtherBodyIndex :type Integer) (bFromSweep :type Boolean) (SweepResult :type "HitResult Structure (by ref)"))
  (bind _returnvalue (`self.GetComponentByClass` OtherActor "/Game/BluePrint/Trap_Map_1/ac_钩索/ac_钩索.ac_钩索_C"))
  (`/Engine/EditorBlueprintResources/StandardMacros.IsValid` _returnvalue
    (:`Is Valid`
      (`/Game/BluePrint/Trap_Map_1/ac_钩索/ac_钩索.添加到组件` _returnvalue self))))

(event `self.Sphere1.OnComponentEndOverlap`
  (params (OverlappedComponent :type "PrimitiveComponent Object Reference") (OtherActor :type "Actor Object Reference") (OtherComp :type "PrimitiveComponent Object Reference") (OtherBodyIndex :type Integer))
  (bind _returnvalue (`self.GetComponentByClass` OtherActor "/Game/BluePrint/Trap_Map_1/ac_钩索/ac_钩索.ac_钩索_C"))
  (`/Engine/EditorBlueprintResources/StandardMacros.IsValid` _returnvalue
    (:`Is Valid`
      (`/Game/BluePrint/Trap_Map_1/ac_钩索/ac_钩索.从组件移除` _returnvalue self))))

(event `设为目标锚点`
  (`PrimitiveComponent.SetMaterial` (`self.Sphere`) 0 "/Game/BluePrint/Trap_Map_1/ac_钩索/2.2"))

(event `退出目标锚点`
  (`PrimitiveComponent.SetMaterial` (`self.Sphere`) 0 "/Game/BluePrint/Trap_Map_1/ac_钩索/1.1"))

(fn `UserConstructionScript`)