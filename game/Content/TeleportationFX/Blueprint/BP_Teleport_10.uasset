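; BP_Teleport_10 is an actor that plays a repeating teleportation visual effect on a skeletal mesh with a looping walk animation, without moving the actor.
; A timeline drives the material's dissolve, vertex-noise strength and color opacity, while delayed branches spawn start and end Niagara systems at the actor's location.
; A delayed call to the custom event restarts the sequence.
; The construction script tints the mesh materials with the teleport color.
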(event `CustomEvent`
  (bind _scale_niagara (`self.Scale_Niagara`))
  (`KismetSystemLibrary.Delay` 1.0 :!label _label)
  (`SkeletalMeshComponent.PlayAnimation` (`self.SkeletalMesh`) "/Game/TeleportationFX/Demo/Characters/Mannequins/Animations/Manny/MM_Walk_Fwd.MM_Walk_Fwd" true)
  (`|ExecutionSequence`
    (:`then_0`
      (bind (_direction _dissolve _strength_vertexnoise _color_opacity) (`Timeline|Timeline` :!via `PlayFromStart`)
        (:`Update`
          (`MeshComponent.SetScalarParameterValueOnMaterials` (`self.SkeletalMesh`) "Dissolve" _dissolve)
          (`MeshComponent.SetScalarParameterValueOnMaterials` (`self.SkeletalMesh`) "strength_VN" _strength_vertexnoise)
          (`MeshComponent.SetScalarParameterValueOnMaterials` (`self.SkeletalMesh`) "color Opacity" _color_opacity)
          (`KismetSystemLibrary.Delay` 4.0)
          (`self.CustomEvent`))))
    (:`then_1`
      (`KismetSystemLibrary.Delay` 0.8)
      (`NiagaraFunctionLibrary.SpawnSystemAtLocation` (`self.Niagara`) (`self.K2_GetActorLocation`) (struct) _scale_niagara))
    (:`then_2`
      (`KismetSystemLibrary.Delay` 3.3)
      (`NiagaraFunctionLibrary.SpawnSystemAtLocation` (`self.End_Teleport`) (`self.K2_GetActorLocation`) (struct) _scale_niagara))))

(event `self.ReceiveBeginPlay`
  (goto _label))

(fn `UserConstructionScript`
  (locals (NewLocalVar :type "Vector Structure" :default (0.0 0.0 0.0)))
  (`MeshComponent.SetVectorParameterValueOnMaterials` (`self.SkeletalMesh`) "Color" (`self.Color Teleport`)))